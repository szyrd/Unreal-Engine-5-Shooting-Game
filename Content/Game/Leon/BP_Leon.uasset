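; BP_Leon is the player character for a third-person, Resident Evil-style shooter, handling movement, camera, combat, inventory and interaction.
; It spawns a socketed pistol plus weapon, health and inventory widgets, with the inventory pausing the game.
; Aiming switches to controller-facing rotation and timeline-blends the spring arm over the shoulder, gating firing; ammo lives in maps keyed by weapon type.
; An overlap trigger selects the prompted interactable, while item functions delegate storage to the inventory widget.
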(event `self.ReceiveBeginPlay`
  (`EnhancedInputSubsystemInterface.AddMappingContext` (pcsubsystem `EnhancedInputLocalPlayerSubsystem` (`GameplayStatics.GetPlayerController` 0)) "/Game/Game/Leon/Input/IMC_Leon.IMC_Leon" 0 (struct))
  (bind _returnvalue (`|SpawnActorFromClass` "/Game/Game/Blueprints/Weapon/BP_Pistol.BP_Pistol_C" (`KismetMathLibrary.MakeTransform` (0.0 0.0 0.0)) "Undefined" "MultiplyWithRoot" null null))
  (bind _output_get (set `self.Weapon Ref` _returnvalue))
  (`self.K2_AttachToComponent` _output_get (`self.Mesh`) "GunSocket" "KeepRelative" "KeepRelative" "KeepRelative" true)
  (bind _returnvalue_2 (`|CreateWidget` "/Game/Game/Blueprints/Weapon/UI_Pistol.UI_Pistol_C" null self))
  (set `self.Weapon UI` _returnvalue_2)
  (`UserWidget.AddToViewport` (`self.Weapon UI`) 0)
  (bind _returnvalue_3 (`|CreateWidget` "/Game/Game/Leon/UI_LeonHUD.UI_LeonHUD_C"))
  (bind _output_get_2 (set `self.UI Health` _returnvalue_3))
  (`UserWidget.AddToViewport` _output_get_2 0)
  (`/Game/Game/Leon/UI_LeonHUD.Update Health UI` (`self.UI Health`))
  (bind _returnvalue_4 (`|CreateWidget` "/Game/Game/Blueprints/InventorySystem/UI_InventoryMenu.UI_InventoryMenu_C"))
  (bind _output_get_3 (set `self.UI Inventory` _returnvalue_4))
  (`UserWidget.AddToViewport` _output_get_3 0)
  (`Widget.RemoveFromParent` (`self.UI Inventory`)))

(event `EnhancedInput|/Game/Game/Leon/Input/IA_CameraControl`
  (params (ActionValue :type "Vector2D Structure") (ElapsedSeconds :type "Float (double-precision)") (TriggeredSeconds :type "Float (double-precision)") (InputAction :type "InputAction Object Reference" :default "/Game/Game/Leon/Input/IA_CameraControl.IA_CameraControl"))
  (bind (_x _y) (`KismetMathLibrary.BreakVector2D` ActionValue))
  ;[1 1 1] Camera Control
  (:`Triggered`
    (`self.AddControllerYawInput` _x)
    (bind _output_get (set `self.VerticalLookAngle` (`KismetMathLibrary.FClamp` (+ (* _y (`KismetMathLibrary.SelectFloat` -1.0 1.0 (`self.InverseCameraVertical`))) (`self.VerticalLookAngle`)) -45.0 45.0)))
    (`SceneComponent.K2_SetRelativeRotation` (`self.SpringArm`) (`KismetMathLibrary.MakeRotator` 0.0 _output_get) false false)))

(event `EnhancedInput|/Game/Game/Leon/Input/IA_Inventory`
  (params (ActionValue :type Boolean) (ElapsedSeconds :type "Float (double-precision)") (TriggeredSeconds :type "Float (double-precision)") (InputAction :type "InputAction Object Reference" :default "/Game/Game/Leon/Input/IA_Inventory.IA_Inventory"))
  ;[1 1 1] Inventory
  (:`Started`
    (`UserWidget.AddToViewport` (`self.UI Inventory`) 0)
    (`GameplayStatics.SetGamePaused` true)
    (set `PlayerController.bShowMouseCursor` true (`GameplayStatics.GetPlayerController` 0))
    (`WidgetBlueprintLibrary.SetInputMode_UIOnlyEx` (`GameplayStatics.GetPlayerController` 0) null)))

(event `EnhancedInput|/Game/Game/Leon/Input/IA_Move`
  (params (ActionValue :type "Vector2D Structure") (ElapsedSeconds :type "Float (double-precision)") (TriggeredSeconds :type "Float (double-precision)") (InputAction :type "InputAction Object Reference" :default "/Game/Game/Leon/Input/IA_Move.IA_Move"))
  (bind _returnvalue (`self.GetControlRotation`))
  (bind (_x _y) (`KismetMathLibrary.BreakVector2D` (* (`KismetMathLibrary.Normal2D` ActionValue) (`KismetMathLibrary.SelectFloat` 1.0 0.6 (and (`|GetInputActionValue`) (not (`self.Is Aiming`)))))))
  ;[1 1 1] Move
  (:`Triggered`
    (if (not (== (`self.PlayerHealth`) 0.0))
      (`self.AddMovementInput` (`KismetMathLibrary.GetRightVector` _returnvalue) _x)
      (`self.AddMovementInput` (`KismetMathLibrary.GetForwardVector` _returnvalue) _y))))

(event `Start Aim`
  (bind _charactermovement (`self.CharacterMovement`))
  (bind _springarm (`self.SpringArm`))
  ;[1 1 1] Aiming
  (if (and (not (== (`self.PlayerHealth`) 0.0)) (`self.Is Aiming`))
    (`/Game/Game/Blueprints/Weapon/UI_Pistol.Show Crosshair` (`self.Weapon UI`) true)
    (set `CharacterMovementComponent.bOrientRotationToMovement` false _charactermovement)
    (set `CharacterMovementComponent.bUseControllerDesiredRotation` true _charactermovement)
    (bind (_direction _float2) (`Timeline|Timeline` :!label _label)
      (:`Update`
        (set `SpringArmComponent.TargetArmLength` (`KismetMathLibrary.Lerp` 80.0 60.0 _float2) _springarm)
        (set `SpringArmComponent.SocketOffset` (`KismetMathLibrary.VLerp` (0.0 30.0 20.0) (0.0 45.0 25.0) _float2) _springarm)))))

(event `Stop Aim`
  (bind _charactermovement (`self.CharacterMovement`))
  ;[1 1 1] Aiming
  (`/Game/Game/Blueprints/Weapon/UI_Pistol.Show Crosshair` (`self.Weapon UI`) false)
  (set `CharacterMovementComponent.bOrientRotationToMovement` true _charactermovement)
  (set `CharacterMovementComponent.bUseControllerDesiredRotation` false _charactermovement)
  (goto _label :!via `Reverse`))

(event `EnhancedInput|/Game/Game/Leon/Input/IA_Aim`
  (params (ActionValue :type Boolean) (ElapsedSeconds :type "Float (double-precision)") (TriggeredSeconds :type "Float (double-precision)") (InputAction :type "InputAction Object Reference" :default "/Game/Game/Leon/Input/IA_Aim.IA_Aim"))
  ;[1 1 1] Aiming
  (:`Started`
    (set `self.Aim Perssed` true)
    (`self.Start Aim`))
  (:`Completed`
    (set `self.Aim Perssed` false)
    (`self.Stop Aim`)))

(event `EnhancedInput|/Game/Game/Leon/Input/IA_Fire`
  (params (ActionValue :type Boolean) (ElapsedSeconds :type "Float (double-precision)") (TriggeredSeconds :type "Float (double-precision)") (InputAction :type "InputAction Object Reference" :default "/Game/Game/Leon/Input/IA_Fire.IA_Fire"))
  (bind _value (`BlueprintMapLibrary.Map_Find` (`self.Ammo in Clip`) (`/Game/Game/Blueprints/Weapon/BP_WeaponBase.WeaponType` (`self.Weapon Ref`))))
  ;[1 1 1] Fire
  (:`Started`
    (if (and (not (`self.Firing Now`)) (`self.Is Aiming`) (> _value 0))
      (`BlueprintMapLibrary.Map_Add` (`self.Ammo in Clip`) (`/Game/Game/Blueprints/Weapon/BP_WeaponBase.WeaponType` (`self.Weapon Ref`)) (- _value 1))
      (`/Game/Game/Blueprints/Weapon/BP_WeaponBase.Shoot` (`self.Weapon Ref`))
      (set `self.Firing Now` true)
      (bind (_direction _shoot_float) (`Timeline|Shoot Timeline` :!via `PlayFromStart`)
        (:`Update`
          (set `self.Shoot Alpha` _shoot_float))
        (:`Finished`
          (set `self.Firing Now` false))))))

(event `EnhancedInput|/Game/Game/Leon/Input/IA_Reload`
  (params (ActionValue :type Boolean) (ElapsedSeconds :type "Float (double-precision)") (TriggeredSeconds :type "Float (double-precision)") (InputAction :type "InputAction Object Reference" :default "/Game/Game/Leon/Input/IA_Reload.IA_Reload"))
  (bind _weapontype (`/Game/Game/Blueprints/Weapon/BP_WeaponBase.WeaponType` (`self.Weapon Ref`)))
  ;[1 1 1] Reload
  (:`Started`
    (if (and (`self.Can Reload`) (< (`BlueprintMapLibrary.Map_Find` (`self.Ammo in Clip`) _weapontype) 10) (> (`BlueprintMapLibrary.Map_Find` (`self.Total Ammo`) _weapontype) 0))
      (`self.Stop Aim`)
      (set `self.Reloading` true)
      (`/Game/Game/Blueprints/Weapon/BP_WeaponBase.Reload SFX` (`self.Weapon Ref`))
      (`self.Reload`))))

(event `Reload Finished`
  ;[1 1 1] Reload
  (set `self.Reloading` false)
  (`self.Reload`)
  (if (`self.Aim Perssed`)
    (`self.Start Aim`)))

(event `self.Interaction Trigger.OnComponentBeginOverlap`
  (params (OverlappedComponent :type "PrimitiveComponent Object Reference") (OtherActor :type "Actor Object Reference") (OtherComp :type "PrimitiveComponent Object Reference") (OtherBodyIndex :type Integer) (bFromSweep :type Boolean) (SweepResult :type "HitResult Structure (by ref)"))
  ;[1 1 1] Interaction
  (bind _asbp_interactable_base (cast `/Game/Game/Blueprints/Interactables/BP_InteractableBase` OtherActor))
  (`/Engine/EditorBlueprintResources/StandardMacros.IsValid` (`self.Interacting Objecr`)
    (:`Is Valid`
      (`/Game/Game/Blueprints/Interactables/BP_InteractableBase.Show Prompt` (`self.Interacting Objecr`) false))
    (:`Is Not Valid`
      _))
  (bind _output_get (set `self.Interacting Objecr` _asbp_interactable_base))
  (`/Game/Game/Blueprints/Interactables/BP_InteractableBase.Show Prompt` _output_get true))

(event `self.Interaction Trigger.OnComponentEndOverlap`
  (params (OverlappedComponent :type "PrimitiveComponent Object Reference") (OtherActor :type "Actor Object Reference") (OtherComp :type "PrimitiveComponent Object Reference") (OtherBodyIndex :type Integer))
  (bind _overlappingactors (`self.GetOverlappingActors` (`self.Interacting Objecr`) "/Game/Game/Blueprints/Interactables/BP_InteractableBase.BP_InteractableBase_C"))
  ;[1 1 1] Interaction
  (bind _asbp_interactable_base (cast `/Game/Game/Blueprints/Interactables/BP_InteractableBase` OtherActor))
  (`/Game/Game/Blueprints/Interactables/BP_InteractableBase.Show Prompt` _asbp_interactable_base false)
  (if (== _asbp_interactable_base (`self.Interacting Objecr`))
    (set `self.Interacting Objecr` null)
    (elif (> (`KismetArrayLibrary.Array_Length` _overlappingactors) 0)
      (bind _asbp_interactable_base_2 (cast `/Game/Game/Blueprints/Interactables/BP_InteractableBase` (`|GetArrayItem` _overlappingactors)))
      (bind _output_get (set `self.Interacting Objecr` _asbp_interactable_base_2))
      (`/Game/Game/Blueprints/Interactables/BP_InteractableBase.Show Prompt` _output_get true))))

(event `EnhancedInput|/Game/Game/Leon/Input/IA_Interact`
  (params (ActionValue :type Boolean) (ElapsedSeconds :type "Float (double-precision)") (TriggeredSeconds :type "Float (double-precision)") (InputAction :type "InputAction Object Reference" :default "/Game/Game/Leon/Input/IA_Interact.IA_Interact"))
  (bind _interacting_objecr (`self.Interacting Objecr`))
  ;[1 1 1] Interaction
  (:`Started`
    (`/Engine/EditorBlueprintResources/StandardMacros.IsValid` _interacting_objecr
      (:`Is Valid`
        (`/Game/Game/Blueprints/Interactables/BP_InteractableBase.Interact` _interacting_objecr)))))

(fn `Can Reload`
  (returns (`Can Reloead` :type Boolean))
  (bind _weapontype (`/Game/Game/Blueprints/Weapon/BP_WeaponBase.WeaponType` (`self.Weapon Ref`)))
  (return (and (not (`self.Firing Now`)) (> (`BlueprintMapLibrary.Map_Find` (`self.Total Ammo`) _weapontype) 0) (!= (`BlueprintMapLibrary.Map_Find` (`self.Ammo in Clip`) _weapontype) (`BlueprintMapLibrary.Map_Find` (`self.Clip size`) _weapontype)))))

(fn `Check Key Item`
  (params (ItemName :type Name))
  (returns (`has Item` :type Boolean))
  (bind _has_item (`/Game/Game/Blueprints/InventorySystem/UI_InventoryMenu.Contains Item ?` (`self.UI Inventory`) ItemName))
  (return _has_item))

(fn `Is Aiming`
  (returns (Aiming :type Boolean))
  (return (and (`self.Aim Perssed`) (not (`self.Reloading`)))))

(fn `Pick Up Item`
  (params (NewItem :type "/Game/Game/Blueprints/Interactables/BP_PickupBase Object Reference"))
  (returns (Success :type Boolean))
  (bind _success (`/Game/Game/Blueprints/InventorySystem/UI_InventoryMenu.Add Item` (`self.UI Inventory`) (`/Game/Game/Blueprints/Interactables/BP_PickupBase.Item Info` NewItem)))
  (return _success))

(fn `Reload`
  (bind _ammo_in_clip (`self.Ammo in Clip`))
  (bind _total_ammo (`self.Total Ammo`))
  (bind _new_ammo (`self.New Ammo`))
  (bind _weapontype (`/Game/Game/Blueprints/Weapon/BP_WeaponBase.WeaponType` (`self.Weapon Ref`)))
  (bind _weapontype_2 (`/Game/Game/Blueprints/Weapon/BP_WeaponBase.WeaponType` (`self.Weapon Ref`)))
  (bind _value (`BlueprintMapLibrary.Map_Find` _total_ammo _weapontype_2))
  (bind _value_2 (`BlueprintMapLibrary.Map_Find` _ammo_in_clip _weapontype_2))
  (set `self.New Ammo` (`KismetMathLibrary.Min` (- (`BlueprintMapLibrary.Map_Find` (`self.Clip size`) _weapontype_2) _value_2) _value))
  (`BlueprintMapLibrary.Map_Add` _ammo_in_clip _weapontype (+ _value_2 _new_ammo))
  (`BlueprintMapLibrary.Map_Add` _total_ammo _weapontype (- _value _new_ammo)))

(fn `Use Item`
  (params (Item :type "/Game/Game/Blueprints/InventorySystem/STRUCT_ItemInfo Structure"))
  (bind _total_ammo (`self.Total Ammo`))
  (bind _playerhealth (`self.PlayerHealth`))
  (bind _weapontype (`/Game/Game/Blueprints/Weapon/BP_WeaponBase.WeaponType` (`self.Weapon Ref`)))
  (bind _value (`BlueprintMapLibrary.Map_Find` _total_ammo _weapontype))
  (switch `name` (`.ItemName_2_0A64474F2F49C77C39C417819E76DADE` (break `/Game/Game/Blueprints/InventorySystem/STRUCT_ItemInfo` Item))
    (:`Green Herb`
      (`KismetSystemLibrary.PrintString` (`KismetStringLibrary.Conv_DoubleToString` _playerhealth))
      (set `self.PlayerHealth` (+ _playerhealth 10.0)))
    (:`Pistol Ammo`
      (`KismetSystemLibrary.PrintString` (`KismetStringLibrary.Conv_IntToString` _value))
      (`BlueprintMapLibrary.Map_Add` _total_ammo _weapontype (+ _value (`.Quantity_8_186482FA504AA8F2B356A9BCA76666BE` (break `/Game/Game/Blueprints/InventorySystem/STRUCT_ItemInfo` (`/Game/Game/Blueprints/InventorySystem/UI_InventorySlot.Stored Item` (`/Game/Game/Blueprints/InventorySystem/UI_InventoryMenu.CurrentSlot` (`self.UI Inventory`))))))))))

(fn `UserConstructionScript`)