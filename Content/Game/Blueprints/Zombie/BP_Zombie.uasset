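; Zombie enemy that spots pawns with PawnSensing, chases the player (BP_Leon) with AIMoveTo and plays a random left or right attack on arrival.
; HitboxOn toggles that hand's hitbox, whose overlap takes player health and triggers a hit reaction, while EndAttack resumes the chase.
; Player damage lowers zombie health, briefly halting it with a reaction montage, or disabling capsule collision and movement at zero.
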(event `self.ReceiveBeginPlay`)

(event `self.PawnSensing.OnSeePawn`
  (params (Pawn :type "Pawn Object Reference"))
  (if (not (`self.Attacking`))
    (`self.Chase Player`)))

(event `Chase Player`
  ;[1 1 1] Chase Player
  (bind _asbp_leon (cast `/Game/Game/Leon/BP_Leon` (`GameplayStatics.GetPlayerPawn` 0)))
  (if (and (not (== (`/Game/Game/Leon/BP_Leon.PlayerHealth` _asbp_leon) 0.0)) (> (`self.Health`) 0.0))
    (`|AIMoveTo` self (0.0 0.0 0.0) (`GameplayStatics.GetPlayerPawn` 0)
      (:`OnSuccess`
        (`self.Attack`)))))

(event `Attack`
  ;[1 1 1] Attack
  (set `self.Attacking` true)
  (set `self.IsRightHand` (`KismetMathLibrary.RandomBool`))
  (`self.PlayAnimMontage` (select `bool` (`self.IsRightHand`) :`false` "/Game/Game/Blueprints/Zombie/Animations/Zombie_Attack_Left_Montage.Zombie_Attack_Left_Montage" :`true` "/Game/Game/Blueprints/Zombie/Animations/Zombie_Attack_Right_Montage.Zombie_Attack_Right_Montage" :!type "AnimMontage Object Reference")))

(event `End Attack`
  ;[1 1 1] Attack
  (set `self.Attacking` false)
  (`self.Chase Player`))

(event `self.ReceiveAnyDamage`
  (params (Damage :type "Float (single-precision)") (DamageType :type "DamageType Object Reference") (InstigatedBy :type "Controller Object Reference") (DamageCauser :type "Actor Object Reference"))
  ;[1 1 1] Damage
  (if (== DamageCauser (`GameplayStatics.GetPlayerPawn` 0))
    (bind _output_get (set `self.Health` (- (`self.Health`) Damage)))
    (if (> _output_get 0.0)
      (`self.PlayAnimMontage` "/Game/Game/Blueprints/Zombie/Animations/Zombie_Reaction_Hit_Montage.Zombie_Reaction_Hit_Montage")
      (set `CharacterMovementComponent.MaxWalkSpeed` 0.0 (`self.CharacterMovement`))
      (`KismetSystemLibrary.RetriggerableDelay` 2.0)
      (set `CharacterMovementComponent.MaxWalkSpeed` 100.0 (`self.CharacterMovement`))
      (else
        (`PrimitiveComponent.SetCollisionEnabled` (`self.CapsuleComponent`) "NoCollision")
        (set `CharacterMovementComponent.MaxWalkSpeed` 0.0 (`self.CharacterMovement`))))))

(event `self.Left HitBox.OnComponentBeginOverlap`
  (params (OverlappedComponent :type "PrimitiveComponent Object Reference") (OtherActor :type "Actor Object Reference") (OtherComp :type "PrimitiveComponent Object Reference") (OtherBodyIndex :type Integer) (bFromSweep :type Boolean) (SweepResult :type "HitResult Structure (by ref)"))
  ;[1 1 1] Damage
  (if (== OtherActor (`GameplayStatics.GetPlayerPawn` 0))
    (`self.Hurt Player`)))

(event `self.Right HitBox.OnComponentBeginOverlap`
  (params (OverlappedComponent :type "PrimitiveComponent Object Reference") (OtherActor :type "Actor Object Reference") (OtherComp :type "PrimitiveComponent Object Reference") (OtherBodyIndex :type Integer) (bFromSweep :type Boolean) (SweepResult :type "HitResult Structure (by ref)"))
  ;[1 1 1] Damage
  (if (== OtherActor (`GameplayStatics.GetPlayerPawn` 0))
    (`self.Hurt Player`)))

(event `Hurt Player`
  ;[1 1 1] Damage Player
  (bind _asbp_leon (cast `/Game/Game/Leon/BP_Leon` (`GameplayStatics.GetPlayerPawn` 0)))
  (if (not (== (`/Game/Game/Leon/BP_Leon.PlayerHealth` _asbp_leon) 0.0))
    (bind _asbp_leon_2 (cast `/Game/Game/Leon/BP_Leon` (`GameplayStatics.GetPlayerPawn` 0)))
    (bind _playerhealth (`/Game/Game/Leon/BP_Leon.PlayerHealth` _asbp_leon_2))
    (bind _output_get (set `self.bCanBeDamaged` (> _playerhealth 0.0)))
    (bind _output_get_2 (set `/Game/Game/Leon/BP_Leon.PlayerHealth` (- _playerhealth _output_get) _asbp_leon_2))
    (if (> _output_get_2 0.0)
      (`self.PlayAnimMontage` _asbp_leon_2 "/Game/Game/Leon/Animations/Hit_Reaction_Montage.Hit_Reaction_Montage" 1.0 "None")
      (`/Game/Game/Leon/BP_Leon.Stop Aim` _asbp_leon_2)
      (else
        (`self.End Attack`)))))

(fn `HitboxOn`
  (params (On :type Boolean))
  (`PrimitiveComponent.SetCollisionEnabled` (select `bool` (`self.IsRightHand`) :`false` (`self.Left HitBox`) :`true` (`self.Right HitBox`) :!type "PrimitiveComponent Object Reference") (select `bool` On :`false` "NoCollision" :`true` "QueryOnly" :!type "ECollisionEnabled Enum")))

(fn `UserConstructionScript`)