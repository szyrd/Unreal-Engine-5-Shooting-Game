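; BP_GarageDoor is an interactable garage door that slides open and briefly shows itself to the player.
; Its OpenGarageDoor event plays a timeline that lerps the GarageDoor component upward along Z from its closed position.
; Each timeline update also switches the player's view target to the door actor, then after a one-second Delay blends back to the pawn.
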(event `Open Garage Door`
  (bind (_direction _open_track) (`Timeline|OpenGarageDoor`)
    (:`Update`
      (`SceneComponent.K2_SetRelativeLocation` (`self.GarageDoor`) (`KismetMathLibrary.VLerp` (0.0 0.0 0.0) (0.0 0.0 758.033086) _open_track) false false)
      (`PlayerController.SetViewTargetWithBlend` (`GameplayStatics.GetPlayerController` 0) self 0.0 "VTBlend_Linear" 0.0 false)
      (`KismetSystemLibrary.Delay` 1.0)
      (`PlayerController.SetViewTargetWithBlend` (`GameplayStatics.GetPlayerController` 0) (`GameplayStatics.GetPlayerPawn` 0) 1.0 "VTBlend_Linear" 0.0 false))))

(fn `UserConstructionScript`)