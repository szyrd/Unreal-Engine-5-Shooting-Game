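; BP_Door_Locked is a locked door interactable that requires a key item to use.
; It overrides Interact to check the player's BP_Leon pawn for the item matching KeyName.
; With the key, it removes that item from the inventory UI and runs the parent's Interact; without it, it only prints a missing-key message.
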(fn `Interact`
  (bind _asbp_leon (cast `/Game/Game/Leon/BP_Leon` (`GameplayStatics.GetPlayerPawn` 0)))
  (bind _has_item (`/Game/Game/Leon/BP_Leon.Check Key Item` _asbp_leon (`self.KeyName`)))
  (if _has_item
    (`/Game/Game/Blueprints/InventorySystem/UI_InventoryMenu.Remove Item` (`/Game/Game/Leon/BP_Leon.UI Inventory` _asbp_leon) (`self.KeyName`))
    (`parent.Interact`)
    (else
      (`KismetSystemLibrary.PrintString` (`KismetStringLibrary.Concat_StrStr` "Key Item missing" (`KismetStringLibrary.Conv_NameToString` (`self.KeyName`)))))))

(fn `UserConstructionScript`
  (`parent.UserConstructionScript`))