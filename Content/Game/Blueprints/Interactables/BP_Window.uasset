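; BP_Window is an interactable window that briefly moves the player's view to itself.
; Interact calls the Look event, which blends the first player controller's view target to the window, waits on a short Delay, then blends back to the player pawn.
; BeginPlay is disabled and the construction script only calls its parent.
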(event `Look`
  (`PlayerController.SetViewTargetWithBlend` (`GameplayStatics.GetPlayerController` 0) self 1.0 "VTBlend_Linear" 0.0 false)
  (`KismetSystemLibrary.Delay` 2.0)
  (`PlayerController.SetViewTargetWithBlend` (`GameplayStatics.GetPlayerController` 0) (`GameplayStatics.GetPlayerPawn` 0) 1.0 "VTBlend_Linear" 0.0 false))

(fn `Interact`
  (`self.Look`))

(fn `UserConstructionScript`
  (`parent.UserConstructionScript`))