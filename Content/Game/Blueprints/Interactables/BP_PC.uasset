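; BP_PC is an interactable computer that opens the garage doors when the electricity is on.
; Interact calls CheckActivate, then either calls OpenGarageDoor on every BP_GarageDoor in the level or prints that electricity is not activated.
; CheckActivate infers power from a BP_Light's point light color being white, returning on the first light found, so only that one is tested.
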(fn `Check Activate?`
  (returns (actiavted :type Boolean))
  (bind _outactors (`GameplayStatics.GetAllActorsOfClass` "/Game/Game/Blueprints/Interactables/BP_Light.BP_Light_C"))
  (for _array_element _outactors
    (return (== (`LightComponentBase.GetLightColor` (`/Game/Game/Blueprints/Interactables/BP_Light.PointLight` _array_element)) (`KismetMathLibrary.LinearColor_White`)))))

(fn `Interact`
  (bind _actiavted (`self.Check Activate?`))
  (if _actiavted
    (bind _outactors (`GameplayStatics.GetAllActorsOfClass` "/Game/Game/Blueprints/Interactables/BP_GarageDoor.BP_GarageDoor_C"))
    (for _array_element _outactors
      (`/Game/Game/Blueprints/Interactables/BP_GarageDoor.Open Garage Door` _array_element))
    (else
      (`KismetSystemLibrary.PrintString` "Electricity not Activated"))))

(fn `UserConstructionScript`
  (`parent.UserConstructionScript`))