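; BP_FuseBox is an interactable fuse box that restores electricity to the level's lights when the player has the required fuse.
; Interact checks the BP_Leon player pawn for the key item named by FuseName, removing it from the inventory UI if found, or printing a missing-fuse message.
; On success, TurnLightOn finds every BP_Light actor and sets its point light to bright white.
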(event `Turn Light On`
  (bind _outactors (`GameplayStatics.GetAllActorsOfClass` "/Game/Game/Blueprints/Interactables/BP_Light.BP_Light_C"))
  (for _array_element _outactors
    (bind _pointlight (`/Game/Game/Blueprints/Interactables/BP_Light.PointLight` _array_element))
    (`LightComponent.SetLightColor` _pointlight (`KismetMathLibrary.LinearColor_White`) true)
    (`LightComponent.SetIntensity` _pointlight 5000.0)))

(fn `Interact`
  (bind _asbp_leon (cast `/Game/Game/Leon/BP_Leon` (`GameplayStatics.GetPlayerPawn` 0)))
  (bind _has_item (`/Game/Game/Leon/BP_Leon.Check Key Item` _asbp_leon (`self.FuseName`)))
  (if _has_item
    (`/Game/Game/Blueprints/InventorySystem/UI_InventoryMenu.Remove Item` (`/Game/Game/Leon/BP_Leon.UI Inventory` _asbp_leon) (`self.FuseName`))
    (`KismetSystemLibrary.PrintString` "Electricity ON")
    (`self.Turn Light On`)
    (else
      (`KismetSystemLibrary.PrintString` (`KismetStringLibrary.Concat_StrStr` "Fuse missing" (`KismetStringLibrary.Conv_NameToString` (`self.FuseName`)))))))

(fn `UserConstructionScript`
  (`parent.UserConstructionScript`))