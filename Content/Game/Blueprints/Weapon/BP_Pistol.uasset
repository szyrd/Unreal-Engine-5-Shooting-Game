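; Pistol weapon Blueprint providing hitscan firing, fire effects and reload audio as separate functions, with no triggering events of its own.
; LineTrace casts forward from the player camera, spawns a metal impact effect on any blocking hit and applies damage, boosted for "Head" bone hits, which also print a debug string.
; FX plays muzzle flash, camera shake and gunshot sound, while ReloadSFX plays the magazine insert cue.
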(fn `FX`
  (bind _muzzle (`self.Muzzle`))
  (`GameplayStatics.SpawnEmitterAtLocation` "/Game/MilitaryWeapDark/FX/P_Pistol_MuzzleFlash_01.P_Pistol_MuzzleFlash_01" (`SceneComponent.K2_GetComponentLocation` _muzzle) (`SceneComponent.K2_GetComponentRotation` _muzzle))
  (`GameplayStatics.PlayWorldCameraShake` "/Game/Game/Blueprints/Weapon/CS_Pistol.CS_Pistol_C" (`self.K2_GetActorLocation`) 0.0 200.0)
  (`GameplayStatics.PlaySound2D` "/Game/MilitaryWeapDark/Sound/Pistol/PistolB_Fire_Cue.PistolB_Fire_Cue" 1.0 1.0 0.0 null null))

(fn `LineTrace`
  (bind _returnvalue (`GameplayStatics.GetPlayerCameraManager` 0))
  (bind _returnvalue_2 (`self.K2_GetActorLocation` _returnvalue))
  (bind _outhit (`KismetSystemLibrary.LineTraceSingle` _returnvalue_2 (+ _returnvalue_2 (* (`self.GetActorForwardVector` _returnvalue) 10000.0)) "TraceTypeQuery3"))
  (bind (_bblockinghit _binitialoverlap _time _distance _location _impactpoint _normal _impactnormal _physmat _hitactor _hitcomponent _hitbonename) (`GameplayStatics.BreakHitResult` _outhit))
  (if _bblockinghit
    (`GameplayStatics.SpawnEmitterAtLocation` "/Game/MilitaryWeapDark/FX/P_Impact_Metal_Large_01.P_Impact_Metal_Large_01" _impactpoint (`KismetMathLibrary.MakeRotFromX` _impactnormal))
    (bind _returnvalue_3 (== _hitbonename "Head"))
    (`GameplayStatics.ApplyDamage` _hitactor (`KismetMathLibrary.SelectFloat` 50.0 20.0 _returnvalue_3) null (`GameplayStatics.GetPlayerPawn` 0))
    (if _returnvalue_3
      (`KismetSystemLibrary.PrintString` "HeadShot"))))

(fn `Reload SFX`
  (`GameplayStatics.PlaySound2D` "/Game/MilitaryWeapDark/Sound/Pistol/Pistol_ReloadInsert_Cue.Pistol_ReloadInsert_Cue" 1.0 1.0 0.0 null null))

(fn `UserConstructionScript`
  (`parent.UserConstructionScript`))